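; BP_Shield is a game board shield actor that the player drags with the mouse.
; BeginPlay enables click events, and clicking its Cube prints a debug string, sets a drag flag and stores the offset from the cursor hit point.
; While dragged, Tick re-traces under the cursor on the Visibility channel and applies that offset to position the actor in Y and Z only.
; Releasing the left mouse button loops over all BP_Shield actors to clear the drag flag.
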(event OnClicked(Cube)
  (params (TouchedComponent :type Primitive%20Component%20Object%20Reference) (ButtonPressed :type Key%20Structure :default "None"))
  (Development|PrintString "Hello")
  (Variables|Default|SetIsBeingMoved true)
  (Variables|Default|SetMovingOffest (- (Transformation|GetActorLocation) (.Location (Collision|BreakHitResult (.HitResult (Game|Player|GetHitResultUnderCursorbyChannel (Game|GetPlayerController 0) "TraceTypeQuery1" true)))))))

(event EventBeginPlay
  (Variables|/Script/Engine.PlayerController|SetbEnableClickEvents (Game|GetPlayerController 0) true))

(event EventTick
  (params (DeltaSeconds :type Float%20%28single-precision%29))
  (bind _returnvalue (Game|GetPlayerController 0))
  (bind _movingoffest (Variables|Default|GetMovingOffest))
  (bind _hitresult (Game|Player|GetHitResultUnderCursorbyChannel _returnvalue "TraceTypeQuery1" true))
  (bind _location (Collision|BreakHitResult _hitresult))
  (bind _returnvalue_2 (+ _location _movingoffest))
  (bind (_x _y _z) (Math|Vector|BreakVector _returnvalue_2))
  (if (Variables|Default|GetIsBeingMoved)
    (Transformation|SetActorLocation (Math|Vector|MakeVector 0.0 _y _z) false false)))

(event Input|MouseEvents|LeftMouseButton
  (params (Key :type Key%20Structure :default "None"))
  (:Released
    (bind _outactors (Actor|GetAllActorsOfClass "BP_Shield_C"))
    (for _array_element _outactors
      (Variables|Default|SetIsBeingMoved false))))

(fn ConstructionScript)